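; Boss actor that periodically fires projectiles at the player.
; BeginPlay starts a looping timer by function name that calls the BossShoot event at a fixed interval.
; BossShoot spawns BP_BossProjectile at a fixed offset from the boss toward player 0, rotated to face that player, and always spawns regardless of collision.
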(event `BossShoot`
  (`|SpawnActorFromClass` "/Game/_Game/BP_BossProjectile.BP_BossProjectile_C" (`KismetMathLibrary.MakeTransform` (+ (`self.K2_GetActorLocation`) (* (`KismetMathLibrary.Normal` (- (`self.K2_GetActorLocation` (`GameplayStatics.GetPlayerCharacter` 0)) (`self.K2_GetActorLocation`))) 500.0)) (`KismetMathLibrary.FindLookAtRotation` (`self.K2_GetActorLocation`) (`self.K2_GetActorLocation` (`GameplayStatics.GetPlayerCharacter` 0)))) "AlwaysSpawn" "MultiplyWithRoot" null null))

(event `self.ReceiveBeginPlay`
  (`KismetSystemLibrary.K2_SetTimer` null "BossShoot" 2.0 true))

(fn `UserConstructionScript`
  (`parent.UserConstructionScript`))