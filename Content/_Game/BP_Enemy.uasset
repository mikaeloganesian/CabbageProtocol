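; BP_Enemy is a cube-bodied enemy pawn that wanders, chases the first-person player and hurts them on contact.
; A looping timer drives AI movement to random reachable points until PawnSensing spots the player, who then becomes the chase target.
; Cube hits damage and launch the player upward, throttled by a DoOnce cooldown.
; Any damage received removes fixed health; death awards coins through BP_MyGameInstance and turns on cube physics before delayed destruction.
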(event `self.ReceiveAnyDamage`
  (params (Damage :type "Float (single-precision)") (DamageType :type "DamageType Object Reference") (InstigatedBy :type "Controller Object Reference") (DamageCauser :type "Actor Object Reference"))
  (bind _cube (`self.Cube`))
  (set `self.Health` (- (`self.Health`) 50.0))
  (if (<= (`self.Health`) 0.0)
    (bind _asbp_my_game_instance (cast `/Game/_Game/BP_MyGameInstance` (`GameplayStatics.GetGameInstance`)))
    (set `/Game/_Game/BP_MyGameInstance.TotalCoins` (+ (`/Game/_Game/BP_MyGameInstance.TotalCoins` _asbp_my_game_instance) 10) _asbp_my_game_instance)
    (`PrimitiveComponent.SetSimulatePhysics` _cube true)
    (`PrimitiveComponent.SetCollisionProfileName` _cube "PhysicsActor" true)
    (`KismetSystemLibrary.Delay` 2.0)
    (`self.K2_DestroyActor`)))

(event `self.ReceiveBeginPlay`
  (`KismetSystemLibrary.K2_SetTimerDelegate` (delegate `AI_Think`) 1.0 true))

(event `AI_Think`
  (bind _targettochase (`self.TargetToChase`))
  (`/Engine/EditorBlueprintResources/StandardMacros.IsValid` _targettochase
    (:`Is Valid`
      (`|AIMoveTo` self (0.0 0.0 0.0) _targettochase))
    (:`Is Not Valid`
      (`|AIMoveTo` self (`NavigationSystemV1.K2_GetRandomReachablePointInRadius` (`self.K2_GetActorLocation`) 1000.0 null null) null))))

(event `self.PawnSensing.OnSeePawn`
  (params (Pawn :type "Pawn Object Reference"))
  (bind _asbp_first_person_character (cast `/Game/FirstPerson/Blueprints/BP_FirstPersonCharacter` Pawn))
  (set `self.TargetToChase` _asbp_first_person_character))

(event `self.Cube.OnComponentHit`
  (params (HitComponent :type "PrimitiveComponent Object Reference") (OtherActor :type "Actor Object Reference") (OtherComp :type "PrimitiveComponent Object Reference") (NormalImpulse :type "Vector Structure") (Hit :type "HitResult Structure (by ref)"))
  (bind _asbp_first_person_character (cast `/Game/FirstPerson/Blueprints/BP_FirstPersonCharacter` OtherActor))
  (`/Engine/EditorBlueprintResources/StandardMacros.DoOnce` false :!label _label
    (:`Completed`
      (`GameplayStatics.ApplyDamage` _asbp_first_person_character 10.0)
      (`self.LaunchCharacter` _asbp_first_person_character (0.0 0.0 500.0) true true)
      (`KismetSystemLibrary.Delay` 1.0)
      (goto _label :!via `Reset`))))

(event `self.ReceiveTick`
  (params (DeltaSeconds :type "Float (single-precision)")))

(fn `UserConstructionScript`)