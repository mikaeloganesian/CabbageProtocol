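; BP_RoomBase is a combat room that spawns enemies on entry and opens its exit once they are gone.
; The first EntryTrigger overlap moves DoorEntry and spawns a random BP_Enemy or BP_Enemy_Sniper at each ArrowComponent tagged EnemySpawn.
; A looping timer then polls CheckWin, which destroys both exit doors when no BP_Enemy actors remain anywhere in the world.
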(event `CheckWin`
  (bind _outactors (`GameplayStatics.GetAllActorsOfClass` "/Game/_Game/BP_Enemy.BP_Enemy_C"))
  (if (== (`KismetArrayLibrary.Array_Length` _outactors) 0)
    (`KismetSystemLibrary.K2_ClearTimer` null "CheckWin")
    (`ActorComponent.K2_DestroyComponent` (`self.Door_Exit_Right`))
    (`ActorComponent.K2_DestroyComponent` (`self.Door_Exit_Left`))))

(event `self.EntryTrigger.OnComponentBeginOverlap`
  (params (OverlappedComponent :type "PrimitiveComponent Object Reference") (OtherActor :type "Actor Object Reference") (OtherComp :type "PrimitiveComponent Object Reference") (OtherBodyIndex :type Integer) (bFromSweep :type Boolean) (SweepResult :type "HitResult Structure (by ref)"))
  (`/Engine/EditorBlueprintResources/StandardMacros.DoOnce` false
    (:`Completed`
      (`SceneComponent.K2_SetRelativeLocation` (`self.Door_Entry`) (50.0 1000.0 500.0) false false)
      (for _array_element (`self.GetComponentsByTag` "/Script/Engine.ArrowComponent" "EnemySpawn")
        (`|SpawnActorFromClass` (select `bool` (`KismetMathLibrary.RandomBool`) :`false` "/Game/_Game/BP_Enemy.BP_Enemy_C" :`true` "/Game/_Game/BP_Enemy_Sniper.BP_Enemy_Sniper_C" :!type "Actor Class Reference") (`SceneComponent.K2_GetComponentToWorld` _array_element) "Undefined" "MultiplyWithRoot" null null))
      (`KismetSystemLibrary.K2_SetTimer` null "CheckWin" 1.0 true))))

(fn `UserConstructionScript`)